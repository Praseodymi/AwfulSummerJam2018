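; Enemy turret that pops out when the player comes within range, tracks them and fires until its Damageable health runs out, then plays explosion and spark effects.
; One timeline, reversed out of range, drives doors, pole height and the blend into split yaw/pitch aiming.
; Once fully deployed, the indicator turns red and a gate with a delay paces shots.
; Bullets are particles whose collisions spawn a temporary DetectionSphere to damage overlapping Damageable actors.
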(event OnParticleCollide(ParticleSystem)
  (params (EventName :type Name :default "None") (EmitterTime :type Float%20%28single-precision%29) (ParticleTime :type Integer) (Location :type Vector :default "0, 0, 0") (Velocity :type Vector :default "0, 0, 0") (Direction :type Vector :default "0, 0, 0") (Normal :type Vector :default "0, 0, 0") (BoneName :type Name :default "None") (PhysMat :type Physical%20Material%20Object%20Reference))
  ;[1 1 1] Do a thing when the bullet particle hits something
  (bind _returnvalue (Game|SpawnActorfromClass "/Game/Blueprint/DetectionSphere.DetectionSphere_C" (Math|Transform|MakeTransform Location) "Undefined" 0 0))
  (for _array_element (Collision|GetOverlappingActors _returnvalue 0 :!class /Script/Engine.Actor)
    (if true
      (if true
        (if (Utilities|IsValid _array_element)
          (if (Utilities|IsValid (Actor|GetComponentbyClass _array_element "/Game/Blueprint/Enemies/Damageable.Damageable_C"))
            (Default|TakeDamage (Actor|GetComponentbyClass _array_element "/Game/Blueprint/Enemies/Damageable.Damageable_C") (Variables|Default|GetDamage) self "0, 0, 0"))))))
  (Actor|DestroyActor _returnvalue))

(event Custom|Activate
  (bind _poleaxis (Variables|Default|GetPoleAxis))
  (bind _relativelocation (Variables|/Script/Engine.SceneComponent|GetRelativeLocation _poleaxis))
  (bind (_x _y) (Math|Vector|BreakVector _relativelocation))
  (bind (_direction _poleheight _lerp _door1 _door2) (Timeline|Timeline_0 Play)
    (:Update
      (Transformation|SetRelativeLocation _poleaxis (Math|Vector|MakeVector _x _y _poleheight) false false))))

(event Custom|Shoot
  (bind _asfirst_person_character (Utilities|Casting|CastToFirstPersonCharacter (Game|GetPlayerCharacter 0)))
  (if (Default|IsAlive (Variables|/Game/FirstPersonBP/Blueprints/FirstPersonCharacter.FirstPersonCharacter_C|GetPlayerDamagable _asfirst_person_character))
    (Components|Activation|Activate (Variables|Default|GetParticleSystem) false)))

(event Custom|Die
  (Components|Activation|Activate (Variables|Default|GetExplosion) false)
  (Components|Activation|Activate (Variables|Default|GetDeadRobotSparks) false))

(event Custom|Deactivate
  (bind _poleaxis (Variables|Default|GetPoleAxis))
  (bind _relativelocation (Variables|/Script/Engine.SceneComponent|GetRelativeLocation _poleaxis))
  (bind (_x _y) (Math|Vector|BreakVector _relativelocation))
  (bind (_direction _poleheight _lerp _door1 _door2) (Timeline|Timeline_0 Reverse)
    (:Update
      (Transformation|SetRelativeLocation _poleaxis (Math|Vector|MakeVector _x _y _poleheight) false false))))

(event EventBeginPlay
  (EventDispatchers|BindEventtoDie (Variables|Default|GetDamageable) (delegate Custom|Die)))

(event EventTick
  (params (DeltaSeconds :type Float%20%28single-precision%29))
  (bind _returnvalue (Game|GetPlayerCharacter 0))
  (bind _indicator (Variables|Default|GetIndicator))
  (bind _poleaxis (Variables|Default|GetPoleAxis))
  (bind _playerheight (Variables|Default|GetPlayerHeight))
  (bind _barrelaxis (Variables|Default|GetBarrelAxis))
  (bind _returnvalue_2 (Math|Vector|MakeVector 0.0 0.0 _playerheight))
  (bind _relativerotation (Variables|/Script/Engine.SceneComponent|GetRelativeRotation _barrelaxis))
  (bind _capsulecomponent (Variables|/Script/Engine.Character|GetCapsuleComponent _returnvalue))
  (bind _relativerotation_2 (Variables|/Script/Engine.SceneComponent|GetRelativeRotation _poleaxis))
  (bind (_roll _pitch _yaw) (Math|Rotator|BreakRotator _relativerotation))
  (bind _returnvalue_3 (Transformation|GetWorldLocation _capsulecomponent))
  (bind (_roll_2 _pitch_2) (Math|Rotator|BreakRotator _relativerotation_2))
  (bind _returnvalue_4 (+ _returnvalue_3 _returnvalue_2))
  (if (> (Variables|/Game/Blueprint/Enemies/Damageable.Damageable_C|GetHealth (Variables|Default|GetDamageable)) 0)
    (if (<= (Math|Vector|VectorLengthSquared (- (Transformation|GetWorldLocation (Variables|Default|GetDefaultSceneRoot)) (Transformation|GetWorldLocation (Variables|/Script/Engine.Character|GetCapsuleComponent (Game|GetPlayerCharacter 0))))) (Math|Float|Square (Variables|Default|GetRange)))
      (CallFunction|Activate)
      (else
        (CallFunction|Deactivate)))
    (if (> (stale Custom|Activate _lerp) 0.0)
      (Transformation|SetRelativeLocation (Variables|Default|GetTurret_TurretDoor1) (Math|Vector|MakeVector 0.0 (stale Custom|Activate _door1) 0.0) false false)
      (Transformation|SetRelativeLocation (Variables|Default|GetTurret_TurretDoor2) (Math|Vector|MakeVector 0.0 (stale Custom|Activate _door2) 0.0) false false)
      (Transformation|SetRelativeRotation _poleaxis (Math|Rotator|Lerp(Rotator) "0,90.000000, 0" (Math|Rotator|MakeRotator _roll_2 _pitch_2 (.Yaw (Math|Rotator|BreakRotator (Math|Transform|InverseTransformRotation (Transformation|GetWorldTransform (Variables|Default|GetDefaultSceneRoot)) (Math|Rotator|FindLookatRotation (Transformation|GetWorldLocation _poleaxis) _returnvalue_4))))) (stale Custom|Activate _lerp)) false false)
      (Transformation|SetRelativeRotation _barrelaxis (Math|Rotator|Lerp(Rotator) "90.000000,90.000000,0.000000" (Math|Rotator|MakeRotator _roll (.Pitch (Math|Rotator|BreakRotator (Math|Transform|InverseTransformRotation (Transformation|GetWorldTransform (Variables|Default|GetDefaultSceneRoot)) (Math|Rotator|FindLookatRotation (Transformation|GetWorldLocation _barrelaxis) _returnvalue_4)))) _yaw) (stale Custom|Activate _lerp)) false false)
      (if (== (stale Custom|Activate _lerp) 1.0)
        (Rendering|Material|SetMaterial _indicator 0 "/Game/Materials/TurretIndicator_Red.TurretIndicator_Red")
        (Utilities|FlowControl|Gate false :!label _label
          (:Exit
            (Utilities|FlowControl|Sequence
              (:then_0
                (CallFunction|Shoot))
              (:then_1
                (Utilities|FlowControl|Delay (Variables|Default|GetfireRate))
                (goto _label Open))
              (:then_2
                (goto _label Close)))))
        (else
          (Rendering|Material|SetMaterial _indicator 0 "/Game/Materials/TurretIndicator_Green.TurretIndicator_Green"))))))

(fn ConstructionScript)