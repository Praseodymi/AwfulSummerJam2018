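; Damageable Blueprint for enemies that tracks health and death state.
; Its TakeDamage event subtracts damage from Health while it is alive.
; A lethal hit stores the damage owner, sets IsDead and calls the Die dispatcher, while a survived hit calls DamageTaken.
; IsAlive exposes the inverse of the death flag.
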(event Custom|TakeDamage
  (params (Damage :type Integer) (Owner :type Actor%20Object%20Reference))
  (if (not (Variables|Default|GetIsDead))
    (if (> (stale _output_get) 0)
      (bind _output_get (Variables|Default|SetHealth (- (stale _output_get) Damage)))
      (if (<= _output_get 0)
        (Variables|Default|SetLastDamageOwner Owner)
        (Variables|Default|SetIsDead true)
        (Default|CallDie)
        (else
          (Default|CallDamageTaken))))))

(event EventBeginPlay)

(event EventTick
  (params (DeltaSeconds :type Float%20%28single-precision%29)))

(fn IsAlive
  (return (not (Variables|Default|GetIsDead))))