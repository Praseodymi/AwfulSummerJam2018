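; BallBot_W_Particles is an enemy BallBot variant that moves by velocity and runs an EyeballShot effect.
; Each Tick calls the parent, clamps CurrentVelocity to MaxSpeed, then applies a swept, delta-time-scaled location move.
; It also calls Activate on EyeballShot every frame without reset.
; Nothing in this file sets a direction for CurrentVelocity, and the other events are disabled or only call the parent.
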(event EventBeginPlay
  (|CallParentFunction) ; This node is disabled and will not be called.\nDrag off pins to build functionality.
)

(event Collision|EventActorBeginOverlap
  (params (OtherActor :type Actor%20Object%20Reference))
  (|CallParentFunction OtherActor) ; This node is disabled and will not be called.\nDrag off pins to build functionality.
)

(event EventTick
  (params (DeltaSeconds :type Float%20%28single-precision%29))
  (|CallParentFunction DeltaSeconds)
  (bind _output_get (Variables|Default|SetCurrentVelocity (Math|Vector|ClampVectorSize (Variables|Default|GetCurrentVelocity) 0.0 (Variables|Default|GetMaxSpeed))))
  (Transformation|SetActorLocation (+ (* _output_get DeltaSeconds) (Transformation|GetActorLocation)) true false)
  (Components|Activation|Activate (Variables|Default|GetEyeballShot) false))

(fn ConstructionScript
  (|CallParentFunction))