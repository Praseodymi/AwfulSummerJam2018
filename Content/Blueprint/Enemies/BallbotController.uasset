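; BallbotController is the controller for the BallBot enemy, driving it toward a Target actor.
; BeginPlay casts and caches the controlled BallBot pawn.
; Each Tick runs a synchronous navigation path query to Target, then adds the offset from the pawn to the path's last point onto its CurrentVelocity.
; Intermediate waypoints are ignored, and the accumulated velocity is neither normalized nor scaled by delta time.
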(event EventBeginPlay
  (|CallParentFunction)
  (bind _asball_bot (Utilities|Casting|CastToBallBot (Pawn|GetControlledPawn)))
  (Variables|Default|SetBallBotPawn _asball_bot))

(event EventTick
  (params (DeltaSeconds :type Float%20%28single-precision%29))
  (bind _ballbotpawn (Variables|Default|GetBallBotPawn))
  (bind _returnvalue (Class|NavigationSystem|FindPathtoActorSynchronously (Transformation|GetWorldLocation (Variables|/Script/Engine.Actor|GetRootComponent (Variables|Default|GetBallBotPawn))) (Variables|Default|GetTarget) 0.0 self))
  (bind _output_get (Variables|/Game/Blueprint/Enemies/BallBot.BallBot_C|SetCurrentVelocity _ballbotpawn (+ (- (Utilities|Array|Get(acopy) (Variables|/Script/Engine.NavigationPath|GetPathPoints _returnvalue) (- (Utilities|Array|Length (Variables|/Script/Engine.NavigationPath|GetPathPoints _returnvalue)) 1)) (Transformation|GetActorLocation _ballbotpawn)) (stale _output_get)))))

(fn ConstructionScript)