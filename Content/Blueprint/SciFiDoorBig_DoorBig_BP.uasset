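; Big sci-fi double door Blueprint that slides its two panels apart when opened and closes itself automatically.
; Open and Close events use an open-state flag to play or reverse a timeline, with play rate derived from a playback time variable.
; The timeline's height track offsets the left and right panels in opposite directions along X, scaled by each panel's relative scale.
; A three-second Delay triggered from the timeline update calls Close.
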(event Custom|Open
  (bind _doorright (Variables|Default|GetDoorRight))
  (bind _doorleft (Variables|Default|GetDoorLeft))
  (Components|Timeline|SetPlayRate (Variables|Default|GetTimeline_0) (/ 1.0 (Variables|Default|GetPlaybackTime_0)))
  (if (not (Variables|Default|GetIsOpen_0))
    (Variables|Default|SetIsOpen_0 true)
    (bind _height (Timeline|Timeline_0 Play)
      (:Update
        (Transformation|SetRelativeLocation _doorright (Math|Vector|MakeVector (* (* _height 1.7e+02) (.X (Math|Vector|BreakVector (Variables|/Script/Engine.SceneComponent|GetRelativeScale3D _doorright)))) 0.0 0.0) false true)
        (Transformation|SetRelativeLocation _doorleft (Math|Vector|MakeVector (* (* _height -1.7e+02) (.X (Math|Vector|BreakVector (Variables|/Script/Engine.SceneComponent|GetRelativeScale3D _doorleft)))) 0.0 0.0) false true)
        (Utilities|FlowControl|Delay 3.0)
        (CallFunction|Close)))))

(event Custom|Close
  (bind _doorright (Variables|Default|GetDoorRight))
  (bind _doorleft (Variables|Default|GetDoorLeft))
  (Components|Timeline|SetPlayRate (Variables|Default|GetTimeline_0) (/ 1.0 (Variables|Default|GetPlaybackTime_0)))
  (if (Variables|Default|GetIsOpen_0)
    (Variables|Default|SetIsOpen_0 false)
    (bind _height (Timeline|Timeline_0 Reverse)
      (:Update
        (Transformation|SetRelativeLocation _doorright (Math|Vector|MakeVector (* (* _height 1.7e+02) (.X (Math|Vector|BreakVector (Variables|/Script/Engine.SceneComponent|GetRelativeScale3D _doorright)))) 0.0 0.0) false true)
        (Transformation|SetRelativeLocation _doorleft (Math|Vector|MakeVector (* (* _height -1.7e+02) (.X (Math|Vector|BreakVector (Variables|/Script/Engine.SceneComponent|GetRelativeScale3D _doorleft)))) 0.0 0.0) false true)
        (Utilities|FlowControl|Delay 3.0)
        (CallFunction|Close)))))

(fn ConstructionScript)