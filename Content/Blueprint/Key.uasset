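; Key pickup actor that the first-person player collects by touching it.
; On overlap with a FirstPersonCharacter, it passes itself to the character's PickupItem, then shows a found-key message built from its KeyName through the character's TextRef.
; It then destroys itself, and BeginPlay, Tick and the construction script add no logic of their own.
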(event EventBeginPlay
  (|CallParentFunction) ; This node is disabled and will not be called.\nDrag off pins to build functionality.
)

(event Collision|EventActorBeginOverlap
  (params (OtherActor :type Actor%20Object%20Reference))
  (bind _asfirst_person_character (Utilities|Casting|CastToFirstPersonCharacter OtherActor))
  (Default|PickupItem _asfirst_person_character self)
  (Default|ShowText (Variables|/Game/FirstPersonBP/Blueprints/FirstPersonCharacter.FirstPersonCharacter_C|GetTextRef _asfirst_person_character) (Utilities|Array|MakeArray (Utilities|String|Append "Found the " (Variables|Default|GetKeyName) " key.")))
  (Actor|DestroyActor))

(event EventTick
  (params (DeltaSeconds :type Float%20%28single-precision%29))
  (|CallParentFunction DeltaSeconds) ; This node is disabled and will not be called.\nDrag off pins to build functionality.
)

(fn ConstructionScript
  (|CallParentFunction))