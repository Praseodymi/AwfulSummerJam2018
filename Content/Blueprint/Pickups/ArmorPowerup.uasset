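; ArmorPowerup is a pickup actor that grants the player an armor upgrade when touched.
; On overlap with a FirstPersonCharacter it passes itself to the character's PickupItem, shows an upgrade message through the character's TextRef, then destroys itself.
; Tick spins the actor at a constant yaw rate while it waits to be collected.
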(event EventBeginPlay
  (|CallParentFunction) ; This node is disabled and will not be called.\nDrag off pins to build functionality.
)

(event Collision|EventActorBeginOverlap
  (params (OtherActor :type Actor%20Object%20Reference))
  (bind _asfirst_person_character (Utilities|Casting|CastToFirstPersonCharacter OtherActor))
  (Default|PickupItem _asfirst_person_character self)
  (Default|ShowText (Variables|/Game/FirstPersonBP/Blueprints/FirstPersonCharacter.FirstPersonCharacter_C|GetTextRef _asfirst_person_character) (Utilities|Array|MakeArray "You've upgraded your armor!"))
  (Actor|DestroyActor))

(event EventTick
  (params (DeltaSeconds :type Float%20%28single-precision%29))
  (Transformation|AddActorLocalRotation (* "0,60.000000, 0" DeltaSeconds) false false))

(fn ConstructionScript
  (|CallParentFunction))