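; Pickup spawner actor that places a configurable Pickup in the level when play begins.
; On BeginPlay it spawns the Pickup at its scene root's transform and casts it.
; It then pushes its own material, health amount and ammo amount onto the spawned pickup's placeholder mesh, health value and weapon ammo.
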(event EventBeginPlay
  (bind _returnvalue (Game|SpawnActorfromClass "/Game/Blueprint/Pickups/Pickup.Pickup_C" (Transformation|GetWorldTransform (Variables|Default|GetDefaultSceneRoot)) "Undefined" 0 0))
  (bind _aspickup (Utilities|Casting|CastToPickup _returnvalue))
  (Variables|/Game/Blueprint/Pickups/Pickup.Pickup_C|SetplaceholderMesh _aspickup 0)
  (Rendering|Material|SetMaterial (Variables|/Game/Blueprint/Pickups/Pickup.Pickup_C|GetplaceholderMesh _aspickup) 0 (Variables|Default|GetMaterial))
  (Variables|/Game/Blueprint/Pickups/Pickup.Pickup_C|SetHealthValue _aspickup (Variables|Default|GetHealthAmt))
  (Variables|/Game/Blueprint/Pickups/Pickup.Pickup_C|SetWeaponAmmo _aspickup (Variables|Default|GetAmmoAmt)))

(fn ConstructionScript)