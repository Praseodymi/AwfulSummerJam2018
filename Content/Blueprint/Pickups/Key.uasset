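; Key pickup actor whose logic for being collected by the player is present but not connected.
; On overlap it only casts the other actor to FirstPersonCharacter, with nothing wired after the cast.
; A detached, never-executed chain would pass the key to PickupItem, call SavePlayer, show a found message built from KeyName through the character's TextRef, then destroy the actor.
; The construction script just calls its parent.
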(event EventBeginPlay)

(event Collision|EventActorBeginOverlap
  (params (OtherActor :type Actor%20Object%20Reference))
  (bind _asfirst_person_character (Utilities|Casting|CastToFirstPersonCharacter OtherActor)))

(event EventTick
  (params (DeltaSeconds :type Float%20%28single-precision%29)))

(fn ConstructionScript
  (|CallParentFunction))