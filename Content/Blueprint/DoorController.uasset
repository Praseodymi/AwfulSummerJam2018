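; DoorController opens a set of doors once every enemy in its assigned list has died.
; On BeginPlay it binds CheckDeaths to the die event of each enemy's Damageable component.
; Each death triggers a pass that removes invalid or dead enemies from EnemyArray during the forward loop, then calls Open on everything in DoorArray when the list is empty.
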(event Custom|Check%20Deaths
  (bind _enemyarray (Variables|Default|GetEnemyArray))
  (for (_array_element _array_index) _enemyarray
    (if (Utilities|IsValid _array_element)
      (if (not (Default|IsAlive (Actor|GetComponentbyClass _array_element "/Game/Blueprint/Enemies/Damageable.Damageable_C")))
        (Utilities|Array|RemoveIndex _enemyarray _array_index :!label _label))
      (else
        (goto _label))))
  (if (== (Utilities|Array|Length _enemyarray) 0)
    (for _array_element_2 (Variables|Default|GetDoorArray)
      (Default|Open _array_element_2))))

(event EventBeginPlay
  (for _array_element (Variables|Default|GetEnemyArray)
    (EventDispatchers|BindEventtoDie (Actor|GetComponentbyClass _array_element "/Game/Blueprint/Enemies/Damageable.Damageable_C") (delegate Custom|Check%20Deaths))))

(fn ConstructionScript)