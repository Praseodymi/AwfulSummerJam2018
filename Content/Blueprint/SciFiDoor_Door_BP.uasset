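; Sci-fi door Blueprint with top and bottom halves that slide apart vertically on Open and automatically close again.
; A timeline height value drives both halves' relative Z in opposite directions, scaled by each component's scale, with play rate derived from a playback time variable.
; The timeline's update also starts a three-second delay before calling Close, which reverses it.
; An open-state flag guards both events against repeat calls.
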(event Custom|Open
  (bind _doorbottom (Variables|Default|GetDoorBottom))
  (bind _doortop (Variables|Default|GetDoorTop))
  (Components|Timeline|SetPlayRate (Variables|Default|GetTimeline_0_0) (/ 1.0 (Variables|Default|GetPlaybackTime_0)))
  (if (not (Variables|Default|GetIsOpen_0))
    (Variables|Default|SetIsOpen_0 true)
    (bind _height (Timeline|Timeline_0_0 Play)
      (:Update
        (Transformation|SetRelativeLocation _doortop (Math|Vector|MakeVector 0.0 0.0 (* (* _height 1.5e+02) (.Z (Math|Vector|BreakVector (Variables|/Script/Engine.SceneComponent|GetRelativeScale3D _doortop))))) false true)
        (Transformation|SetRelativeLocation _doorbottom (Math|Vector|MakeVector 0.0 0.0 (* (* _height -1.5e+02) (.Z (Math|Vector|BreakVector (Variables|/Script/Engine.SceneComponent|GetRelativeScale3D _doorbottom))))) false true)
        (Utilities|FlowControl|Delay 3.0)
        (CallFunction|Close)))))

(event Custom|Close
  (bind _doorbottom (Variables|Default|GetDoorBottom))
  (bind _doortop (Variables|Default|GetDoorTop))
  (Components|Timeline|SetPlayRate (Variables|Default|GetTimeline_0_0) (/ 1.0 (Variables|Default|GetPlaybackTime_0)))
  (if (Variables|Default|GetIsOpen_0)
    (Variables|Default|SetIsOpen_0 false)
    (bind _height (Timeline|Timeline_0_0 Reverse)
      (:Update
        (Transformation|SetRelativeLocation _doortop (Math|Vector|MakeVector 0.0 0.0 (* (* _height 1.5e+02) (.Z (Math|Vector|BreakVector (Variables|/Script/Engine.SceneComponent|GetRelativeScale3D _doortop))))) false true)
        (Transformation|SetRelativeLocation _doorbottom (Math|Vector|MakeVector 0.0 0.0 (* (* _height -1.5e+02) (.Z (Math|Vector|BreakVector (Variables|/Script/Engine.SceneComponent|GetRelativeScale3D _doorbottom))))) false true)
        (Utilities|FlowControl|Delay 3.0)
        (CallFunction|Close)))))

(fn ConstructionScript)