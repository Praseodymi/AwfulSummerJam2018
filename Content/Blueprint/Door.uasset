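; Door Blueprint that slides a Cube component vertically along its relative Z axis through Open and Close events.
; An IsOpen flag guards a timeline that plays forward to open and reverses to close, with its play rate derived from PlaybackTime.
; The timeline's Height track, multiplied by 100 and the cube's Z scale, sets the swept relative location, so travel follows the door's size.
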(event Custom|Open
  (bind _cube (Variables|Default|GetCube))
  (Components|Timeline|SetPlayRate (Variables|Default|GetTimeline_0) (/ 1.0 (Variables|Default|GetPlaybackTime)))
  (if (not (Variables|Default|GetIsOpen))
    (Variables|Default|SetIsOpen true)
    (bind _height (Timeline|Timeline_0 Play)
      (:Update
        (Transformation|SetRelativeLocation _cube (Math|Vector|MakeVector 0.0 0.0 (* (* _height 1e+02) (.Z (Math|Vector|BreakVector (Variables|/Script/Engine.SceneComponent|GetRelativeScale3D _cube))))) true true)))))

(event Custom|Close
  (bind _cube (Variables|Default|GetCube))
  (Components|Timeline|SetPlayRate (Variables|Default|GetTimeline_0) (/ 1.0 (Variables|Default|GetPlaybackTime)))
  (if (Variables|Default|GetIsOpen)
    (Variables|Default|SetIsOpen false)
    (bind _height (Timeline|Timeline_0 Reverse)
      (:Update
        (Transformation|SetRelativeLocation _cube (Math|Vector|MakeVector 0.0 0.0 (* (* _height 1e+02) (.Z (Math|Vector|BreakVector (Variables|/Script/Engine.SceneComponent|GetRelativeScale3D _cube))))) true true)))))

(fn ConstructionScript)