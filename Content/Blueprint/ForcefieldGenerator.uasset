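; A destructible forcefield generator actor that powers a linked forcefield until it is killed.
; On BeginPlay it binds its death handler to the Die event of its Damageable.
; On death it stops its generator particles, fires three explosion effects, destroys the referenced Forcefield actor and turns its cone and cube meshes gray.
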(event Custom|Die
  (Components|Activation|Deactivate (Variables|Default|GetP_ForcefieldGenerator))
  (Components|Activation|Activate (Variables|Default|GetP_Explosion_Bomb) false)
  (Actor|DestroyActor (Variables|Default|GetForcefield))
  (Rendering|Material|SetMaterial (Variables|Default|GetCone) 0 "/Game/Materials/Gray.Gray"))

(event EventBeginPlay
  (EventDispatchers|BindEventtoDie (Variables|Default|GetDamageable) (delegate Custom|Die)))

(fn ConstructionScript)